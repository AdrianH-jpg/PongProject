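; BP_Bola is the ball actor for the Pong game, moving on the horizontal XY plane.
; On BeginPlay it applies an impulse to its Sphere component, scaled from the actor's current velocity.
; Each Tick it offsets its location by the X and Y variables times DeltaSeconds, with sweep off, so this movement does no collision checks.
; The file contains no bounce or scoring logic.
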(event EventBeginPlay
  (Physics|AddImpulseatLocation (Variables|Default|GetSphere) (* (Transformation|GetVelocity) 1e+02) (Transformation|GetActorLocation) "None"))

(event Collision|EventActorBeginOverlap
  (params (OtherActor :type Actor%20Object%20Reference)))

(event EventTick
  (params (DeltaSeconds :type Float%20%28single-precision%29))
  (Transformation|SetActorLocation (+ (Math|Vector|MakeVector (* DeltaSeconds (Variables|Default|GetX)) (* DeltaSeconds (Variables|Default|GetY)) 0.0) (Transformation|GetActorLocation)) false false))

(fn ConstructionScript)