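; BP_Enemy is the opponent paddle in a Pong game, which tracks the BP_Bola ball found at BeginPlay.
; Each Tick snaps the actor to the ball's X, then clamps the Cube's X within fixed bounds.
; When the ball's Y drops below a threshold a Timeline plays to drive the Cube's Y, and otherwise it reverses.
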(event EventBeginPlay
  (bind _returnvalue (Actor|GetActorOfClass "/Game/PongGame/Blueprint/Actor/BP_Bola.BP_Bola_C"))
  (Variables|References|SetBP_BallRef _returnvalue))

(event EventTick
  (params (DeltaSeconds :type Float%20%28single-precision%29))
  (bind _cube (Variables|Default|GetCube))
  (bind _cube_2 (Variables|Default|GetCube))
  (bind _cube_3 (Variables|Default|GetCube))
  (bind _returnvalue (Transformation|GetWorldLocation _cube_3))
  (bind _returnvalue_2 (Transformation|GetWorldLocation _cube_2))
  (bind _returnvalue_3 (Transformation|GetWorldLocation _cube))
  (bind _returnvalue_4 (Math|Float|Clamp(Float) (.x _returnvalue) -2.5e+02 2.5e+02))
  (Transformation|SetActorLocation (Math|Vector|MakeVector (.x (Transformation|GetWorldLocation (Variables|/Game/PongGame/Blueprint/Actor/BP_Bola.BP_Bola_C|GetSphere (Variables|References|GetBP_BallRef)))) (.y _returnvalue_3) (.z _returnvalue_3)) false false)
  (Transformation|SetWorldLocation (Variables|Default|GetCube) (Math|Vector|MakeVector _returnvalue_4 (.y _returnvalue) (.z _returnvalue)) false false)
  (if (< (.y (Transformation|GetWorldLocation (Variables|/Game/PongGame/Blueprint/Actor/BP_Bola.BP_Bola_C|GetSphere (Variables|References|GetBP_BallRef)))) -6e+01)
    (bind _newtrack_0 (Timeline|Timeline Play)
      (:Update
        (Transformation|SetWorldLocation (Variables|Default|GetCube) (Math|Vector|MakeVector _returnvalue_4 _newtrack_0 (.z _returnvalue_2)) false false)))
    (else
      (Timeline|Timeline Reverse))))

(fn ConstructionScript)