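; BP_Raquetas is the player-controlled paddle Blueprint for the Pong game, moving a Cube component from axis input.
; MoveForwardBackward offsets the cube along local X, then clamps world Y and pins world Z to a fixed height.
; MoveUpDown offsets it along local Z, then clamps world X.
; BeginPlay caches a reference to the BP_Bola ball, which these graphs do not use further.
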(event EventBeginPlay
  (bind _returnvalue (Actor|GetActorOfClass "/Game/PongGame/Blueprint/Actor/BP_Bola.BP_Bola_C"))
  (Variables|Default|SetBP_BallRef _returnvalue))

(event Collision|EventActorBeginOverlap
  (params (OtherActor :type Actor%20Object%20Reference)))

(event EventTick
  (params (DeltaSeconds :type Float%20%28single-precision%29)))

(event Input|AxisEvents|InputAxisMoveUpDown
  (params (AxisValue :type Float%20%28single-precision%29))
  (bind _cube (Variables|Default|GetCube))
  (bind _returnvalue (Transformation|GetWorldLocation _cube))
  (Transformation|AddLocalOffset (Variables|Default|GetCube) (Math|Vector|MakeVector 0.0 0.0 (* AxisValue 4.0)) false false)
  (Transformation|SetWorldLocation (Variables|Default|GetCube) (Math|Vector|MakeVector (Math|Float|Clamp(Float) (.x _returnvalue) -2.5e+02 2.5e+02) (.y _returnvalue) (.z _returnvalue)) false false))

(event Input|AxisEvents|InputAxisMoveForwardBackward
  (params (AxisValue :type Float%20%28single-precision%29))
  (bind _cube (Variables|Default|GetCube))
  (bind _returnvalue (Transformation|GetWorldLocation _cube))
  (Transformation|AddLocalOffset (Variables|Default|GetCube) (Math|Vector|MakeVector (* AxisValue 4.0) 0.0 0.0) false false)
  (Transformation|SetWorldLocation (Variables|Default|GetCube) (Math|Vector|MakeVector (.x _returnvalue) (Math|Float|Clamp(Float) (.y _returnvalue) 3.5e+02 585.0) 3e+01) false false))

(fn ConstructionScript)